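; Attack component shared by the player and enemy characters, handling combo attacks, hit detection, projectiles and summons.
; Grounded attacks step through a montage array, with notifies controlling combo windows, player stamina cost, projectile throws and random summons.
; TriggerComplexHit sphere-traces between melee sockets, ignoring fellow enemies for enemy owners, and applies the owner's attack stat as damage.
; Player blocks convert hits into stamina loss and knock back sword enemies, which then attack again.
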(event Custom|Attack
  (bind _owner (Variables|Default|GetOwner))
  (if (Variables|Default|GetbCanAttack)
    (Variables|Default|SetbCanAttack false)
    (if (not (AI|Components|NavMovement|IsFalling (Variables|/Script/Engine.Character|GetCharacterMovement (Variables|Default|GetOwner))))
      (bind _notifyname (Animation|Montage|PlayMontage (Variables|/Script/Engine.Character|GetMesh (Variables|Default|GetOwner)) (Utilities|Array|Get(acopy) (Variables|Default|GetAttackAnimation) (Variables|Default|GetAtkIndexCurrent)))
        (:then
          (Variables|Default|SetAtkIndexCurrent (Math|Integer|SelectInt (+ (Variables|Default|GetAtkIndexCurrent) 1) 0 (< (Variables|Default|GetAtkIndexCurrent) (Variables|Default|GetAtkIndexMax)))))
        (:OnCompleted
          (Variables|Default|SetAtkIndexCurrent 0)
          (Variables|Default|SetbCanAttack true))
        (:OnNotifyBegin
          (switch name _notifyname
            (:Hit
              (if (== (Utilities|GetClass _owner) "/Game/BP_PlayableCharacter.BP_PlayableCharacter_C")
                ;[1 1 1] Losong stamina
                (bind _asbp_playable_character (Utilities|Casting|CastToBP_PlayableCharacter _owner))
                (Variables|/Game/BP_PlayableCharacter.BP_PlayableCharacter_C|SetStamina _asbp_playable_character (- (Variables|/Game/BP_PlayableCharacter.BP_PlayableCharacter_C|GetStamina _asbp_playable_character) (Variables|/Game/BP_PlayableCharacter.BP_PlayableCharacter_C|GetatkStamina _asbp_playable_character)))))
            (:CanCombo
              (Variables|Default|SetbCanAttack true))
            (:Recovery
              (Variables|Default|SetbCanAttack false))
            (:Throw
              ;[1 1 1] range atk
              (bind _asenemy_distance (Utilities|Casting|CastToEnemyDistance (Variables|Default|GetOwner)))
              (Game|SpawnActorfromClass "/Game/EnemyArchitectur/Range_Enemy/Projectile.Projectile_C" (Math|Transform|MakeTransform (Transformation|GetWorldLocation (Variables|/Game/EnemyArchitectur/Range_Enemy/EnemyDistance.EnemyDistance_C|GetprojectileSpawner _asenemy_distance)) (Transformation|GetWorldRotation (Variables|/Game/EnemyArchitectur/Range_Enemy/EnemyDistance.EnemyDistance_C|GetprojectileSpawner _asenemy_distance)) "0.200000,0.200000,0.200000") "Undefined" 0 0))
            (:Summon
              (CallFunction|Summon)))))
      (else
        (Variables|Default|SetbCanAttack true)))))

(event Custom|beknoc
  ;[1 1 1] play the knock animation on the enemy
  (bind _asenemy_sword (Utilities|Casting|CastToEnemySword (Variables|Default|GetOwner)))
  (Animation|Montage|PlayMontage (Variables|/Script/Engine.Character|GetMesh _asenemy_sword) "/Game/All_Animation/Enemy_Animation/knockback.knockback"
    (:OnCompleted
      (Variables|Default|SetAtkIndexCurrent 0)
      (Variables|Default|SetbCanAttack true)
      (CallFunction|Attack))))

(event EventBeginPlay
  (bind _ascharacter (Utilities|Casting|CastToCharacter (Components|GetOwner)))
  (Variables|Default|SetOwner _ascharacter)
  (Variables|Default|SetAtkIndexMax (- (Utilities|Array|Length (Variables|Default|GetAttackAnimation)) 1)))

(event EventTick
  (params (DeltaSeconds :type Float%20%28single-precision%29)))

(fn TriggerSimpleHit
  ;[1 1 1] simple dmg mechanics
)

(fn TriggerComplexHit
  (bind _owner (Variables|Default|GetOwner))
  (bind _owner_2 (Variables|Default|GetOwner))
  (bind _mesh (Variables|/Script/Engine.Character|GetMesh _owner))
  (bind _mesh_2 (Variables|/Script/Engine.Character|GetMesh _owner_2))
  (if (Utilities|ClassIsChildOf (Utilities|GetClass _owner_2) "/Game/EnemyArchitectur/Parent/Enemy.Enemy_C")
    ;[1 1 1] enemy can't hit enemy
    (bind _outactors (Actor|GetAllActorsOfClass "/Game/EnemyArchitectur/Parent/Enemy.Enemy_C"))
    (bind (_outhit _returnvalue) (Collision|SphereTraceForObjects (Transformation|GetSocketLocation _mesh "SocketMeleStart") (Transformation|GetSocketLocation _mesh "SocketMeleEnd") 0.0 (Utilities|Array|MakeArray "ObjectTypeQuery3") false _outactors "None"))
    (if _returnvalue
      (if (== (Utilities|GetClass (.HitActor (Collision|BreakHitResult _outhit))) "/Game/BP_PlayableCharacter.BP_PlayableCharacter_C")
        (bind _asbp_playable_character (Utilities|Casting|CastToBP_PlayableCharacter (.HitActor (Collision|BreakHitResult _outhit))))
        (if (Variables|/Game/BP_PlayableCharacter.BP_PlayableCharacter_C|GetisBlock _asbp_playable_character)
          (bind _atk (CallFunction|GetAtk))
          (bind _output_get (Variables|/Game/BP_PlayableCharacter.BP_PlayableCharacter_C|SetStamina _asbp_playable_character (- (Variables|/Game/BP_PlayableCharacter.BP_PlayableCharacter_C|GetStamina _asbp_playable_character) (* _atk 1.5))))
          (CallFunction|Beknoc)
          (if (<= _output_get 0.0)
            (Variables|/Game/BP_PlayableCharacter.BP_PlayableCharacter_C|SetStamina _asbp_playable_character 0.0)
            (Variables|/Game/BP_PlayableCharacter.BP_PlayableCharacter_C|SetisBlock _asbp_playable_character false))
          (elif (Variables|/Script/Engine.Actor|GetbCanBeDamaged (.HitActor (Collision|BreakHitResult _outhit)))
            (bind _atk_2 (CallFunction|GetAtk))
            (Game|Damage|ApplyDamage (.HitActor (Collision|BreakHitResult _outhit)) _atk_2 0 0)))))
    (else
      (bind (_outhit_2 _returnvalue_2) (Collision|SphereTraceForObjects (Transformation|GetSocketLocation _mesh_2 "SocketMeleStart") (Transformation|GetSocketLocation _mesh_2 "SocketMeleEnd") 0.0 (Utilities|Array|MakeArray "ObjectTypeQuery3") false 0 "Persistent"))
      (if _returnvalue_2
        (if (== (Utilities|GetClass (.HitActor (Collision|BreakHitResult _outhit_2))) "/Game/BP_PlayableCharacter.BP_PlayableCharacter_C")
          (bind _asbp_playable_character_2 (Utilities|Casting|CastToBP_PlayableCharacter (.HitActor (Collision|BreakHitResult _outhit_2))))
          (if (Variables|/Game/BP_PlayableCharacter.BP_PlayableCharacter_C|GetisBlock _asbp_playable_character_2)
            (bind _atk_3 (CallFunction|GetAtk))
            (Variables|/Game/BP_PlayableCharacter.BP_PlayableCharacter_C|SetStamina _asbp_playable_character_2 (- (Variables|/Game/BP_PlayableCharacter.BP_PlayableCharacter_C|GetStamina _asbp_playable_character_2) (* _atk_3 1.5)))
            (CallFunction|Beknoc)
            (else
              (if (Variables|/Script/Engine.Actor|GetbCanBeDamaged (.HitActor (Collision|BreakHitResult _outhit_2))) :!label _label
                (bind _atk_4 (CallFunction|GetAtk))
                (Game|Damage|ApplyDamage (.HitActor (Collision|BreakHitResult _outhit_2)) _atk_4 0 0))))
          (else
            (goto _label)))))))

(fn Summon
  ;[1 1 1] summon a random enemy in the owner array
  (bind _asenemy_summoner (Utilities|Casting|CastToEnemySummoner (Variables|Default|GetOwner)))
  (Game|SpawnActorfromClass (.OutItem (Utilities|Array|Random (Variables|/Game/EnemyArchitectur/Summoner_Enemy/EnemySummoner.EnemySummoner_C|GetActorToSummon _asenemy_summoner))) (Math|Transform|MakeTransform (Transformation|GetWorldLocation (Variables|/Game/EnemyArchitectur/Summoner_Enemy/EnemySummoner.EnemySummoner_C|GetSummonPlace _asenemy_summoner)) (Transformation|GetWorldRotation (Variables|/Game/EnemyArchitectur/Summoner_Enemy/EnemySummoner.EnemySummoner_C|GetSummonPlace _asenemy_summoner)) "1.000000,1.000000,1.000000") "Undefined" 0 0))

(fn GetAtk
  (bind _owner (Variables|Default|GetOwner))
  (if (Utilities|ClassIsChildOf (Utilities|GetClass (Variables|Default|GetOwner)) "/Game/EnemyArchitectur/Parent/Enemy.Enemy_C")
    (bind _asenemy (Utilities|Casting|CastToEnemy _owner))
    (bind _output_get (Variables|Default|SetStat_Atk (Variables|/Game/EnemyArchitectur/Parent/Enemy.Enemy_C|GetAtk _asenemy)))
    (return _output_get)
    (else
      (bind _asbp_playable_character (Utilities|Casting|CastToBP_PlayableCharacter _owner))
      (bind _output_get_2 (Variables|Default|SetStat_Atk (Variables|/Game/BP_PlayableCharacter.BP_PlayableCharacter_C|GetAtk_Use _asbp_playable_character)))
      (return _output_get_2))))